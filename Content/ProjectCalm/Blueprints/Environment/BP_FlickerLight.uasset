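; BP_FlickerLight is an environment light that flickers its spot light on and off at irregular intervals.
; From BeginPlay, an endless delay loop toggles the spot light component's visibility, without propagating to children, after random waits drawn from separate on-time and off-time ranges.
; Each toggle is guarded by a validity check, so the loop stops if the component becomes invalid.
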(event `self.ReceiveBeginPlay`
  (bind _spotlightcomponent (`self.SpotLightComponent`))
  (`KismetSystemLibrary.Delay` (`KismetMathLibrary.RandomFloatInRange` (`self.MinTimeOn`) (`self.MaxTimeOn`)) :!label _label)
  (`/Engine/EditorBlueprintResources/StandardMacros.IsValid` _spotlightcomponent
    (:`Is Valid`
      (`SceneComponent.ToggleVisibility` _spotlightcomponent false)
      (`KismetSystemLibrary.Delay` (`KismetMathLibrary.RandomFloatInRange` (`self.MinTimeOff`) (`self.MaxTimeOff`)))
      (`/Engine/EditorBlueprintResources/StandardMacros.IsValid` _spotlightcomponent
        (:`Is Valid`
          (`SceneComponent.ToggleVisibility` _spotlightcomponent false)
          (goto _label))))))

(fn `UserConstructionScript`)